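; Player pawn for an object-moving level: an editor-style fly camera that moves and rotates objects implementing ITransform.
; Left-click traces under the cursor to store the object and hit axis component; W and E switch between move and rotate modes.
; While held, Tick turns input into axis-constrained transforms, using dot products against view vectors to set drag sign and weighting.
; Otherwise input turns the camera, and holding right mouse enables flying.
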(event EventBeginPlay
  (Variables|/Script/Engine.PlayerController|SetbShowMouseCursor (Game|GetPlayerController 0) true))

(event Collision|EventActorBeginOverlap
  (params (OtherActor :type Actor%20Object%20Reference)))

(event EventTick
  (params (DeltaSeconds :type Float%20%28single-precision%29))
  (if (Variables|CharacterControl|GetisPressActor)
    (switch int (Variables|Default|GettransformMode)
      (:0
        (CallFunction|HandleActorMove))
      (:1
        (CallFunction|HandleActorRotation (Variables|Other|GetcurrentAxis))))
    (else
      ;[1 1 1] Camera Control
      (Pawn|Input|AddControllerPitchInput (* (Class|Actor|GetInputAxisKeyValue) -1.0))
      (Pawn|Input|AddControllerYawInput (Class|Actor|GetInputAxisKeyValue)))))

(event Input|KeyboardEvents|W
  (params (Key :type Key%20Structure :default "None"))
  (:Pressed
    (if (not (Variables|Default|GetisPressMouseRight))
      (Variables|Default|SettransformMode 0))))

(event Input|KeyboardEvents|E
  (params (Key :type Key%20Structure :default "None"))
  (:Pressed
    (if (not (Variables|Default|GetisPressMouseRight))
      (Variables|Default|SettransformMode 1))))

(event Input|MouseEvents|RightMouseButton
  (params (Key :type Key%20Structure :default "None"))
  (:Pressed
    (Variables|Default|SetisPressMouseRight true))
  (:Released
    (Variables|Default|SetisPressMouseRight false)))

(event Input|MouseEvents|LeftMouseButton
  (params (Key :type Key%20Structure :default "None"))
  ;[1 1 1] 原  点击处理
  (:Pressed
    (Variables|CharacterControl|SetisPressActor true)
    (bind _hitresult (CallFunction|LineTracefromMouseClick))
    ;;[1 1 1] 判断是否带有ITransform接口，若是则能进行变换
    (Development|PrintString (Utilities|String|Append "The name that actor is onHitted is  " (Utilities|GetObjectName (.HitComponent (Collision|BreakHitResult _hitresult)))))
    (bind _asitransform (Utilities|Casting|CastToITransform (.HitActor (Collision|BreakHitResult _hitresult)))
      (:then
        (Variables|Other|SetcurrentAxis (Utilities|GetObjectName (.HitComponent (Collision|BreakHitResult _hitresult))))
        (Variables|Other|SetcurrentSelect _asitransform)
        (Variables|Default|SethitComponent (.HitComponent (Collision|BreakHitResult _hitresult)))
        (Development|PrintString (Utilities|String|ToString(Float) (Math|Vector|DotProduct (Math|Vector|GetForwardVector (.HitComponent (Collision|BreakHitResult _hitresult))) (Math|Vector|GetRightVector (Variables|Default|GetCamera))))))
      (:CastFailed
        (Development|PrintString "This is not ITransform" false)
        (Variables|Other|SetcurrentSelect 0)
        (Variables|Default|SethitComponent 0))))
  (:Released
    (Variables|CharacterControl|SetisPressActor false)
    (Variables|Other|SetcurrentAxis "")))

(fn ConstructionScript)

(fn LineTracefromMouseClick
  (bind _defaultsceneroot (Variables|Default|GetDefaultSceneRoot))
  (bind _returnvalue (Transformation|GetWorldLocation _defaultsceneroot))
  (bind (_outhit _returnvalue_2) (Collision|LineTraceByChannel _returnvalue (+ _returnvalue (* (.WorldDirection (Game|Player|ConvertMouseLocationToWorldSpace (Game|GetPlayerController 0))) 1e+08)) "TraceTypeQuery1" false 0 "None"))
  (return _outhit _returnvalue_2))

(fn HandleActorRotation
  (params (SelectAxis :type String))
  (Utilities|IsValid (Utilities|ToObject(Interface) (Variables|Other|GetcurrentSelect))
    (:Is%20Valid
      (switch string SelectAxis
        (:AxisX
          (LocalVariables|SettempRotator "0, 0,1.000000"))
        (:AxisY
          (LocalVariables|SettempRotator "1.000000, 0, 0"))
        (:AxisZ
          (LocalVariables|SettempRotator "0,1.000000, 0")))
      (Default|SetITransformRotate (Variables|Other|GetcurrentSelect) (LocalVariables|GettempRotator) (Math|Float|Truncate (+ (* (Class|Actor|GetInputAxisKeyValue) 1e+01) (* (Class|Actor|GetInputAxisKeyValue) 5.0)))))
    (:Is%20Not%20Valid
      (Development|PrintString "Not thing can controll" false))))

(fn HandleActorMove
  (Utilities|IsValid (Utilities|ToObject(Interface) (Variables|Other|GetcurrentSelect))
    (:Is%20Valid
      (if (> (Math|Vector|DotProduct (Transformation|GetActorUpVector) (Math|Vector|GetForwardVector (Variables|Default|GethitComponent))) 0.0)
        (LocalVariables|SetisReverseVertical 1.0)
        (else
          (LocalVariables|SetisReverseVertical -1.0)))
      (if (> (Math|Vector|DotProduct (Transformation|GetActorRightVector) (Math|Vector|GetForwardVector (Variables|Default|GethitComponent))) 0.0)
        (LocalVariables|SetisReverseHorizontal 1.0)
        (else
          (LocalVariables|SetisReverseHorizontal -1.0)))
      (bind (_xweight _yweight) (CallFunction|SetXandYAxisWeight))
      (Default|Move (Variables|Other|GetcurrentSelect) (Math|Vector|GetForwardVector (Variables|Default|GethitComponent)) (+ (* _xweight (Class|Actor|GetInputAxisKeyValue) (LocalVariables|GetisReverseHorizontal)) (* (Class|Actor|GetInputAxisKeyValue) (LocalVariables|GetisReverseVertical) _yweight))))
    (:Is%20Not%20Valid
      (Development|PrintString "Not thing can controll" false))))

(fn SetXandYAxisWeight
  (bind _hitcomponent (Variables|Default|GethitComponent))
  (bind _camera (Variables|Default|GetCamera))
  (bind _returnvalue (Math|Vector|GetForwardVector _hitcomponent))
  (bind _returnvalue_2 (Math|Vector|GetRightVector _camera))
  (bind _returnvalue_3 (Math|Vector|DotProduct _returnvalue_2 _returnvalue))
  (if (<= _returnvalue_3 0.5)
    (if (>= _returnvalue_3 -0.5)
      (LocalVariables|SetDecreasedXWeight 0.2)
      (else
        (LocalVariables|SetDecreasedYWeight 0.2 :!label _label)))
    (else
      (goto _label)))
  (return (LocalVariables|GetDecreasedXWeight) (LocalVariables|GetDecreasedYWeight)))

(event Input|AxisEvents|InputAxisInputForward
  (params (AxisValue :type Float%20%28single-precision%29))
  (if (not (Variables|CharacterControl|GetisPressActor))
    (if (Variables|Default|GetisPressMouseRight)
      (Transformation|AddActorWorldOffset (* (* (Math|Transform|TransformDirection (Transformation|GetActorTransform) "1.000000, 0, 0") AxisValue) 15.0)))))

(event Input|AxisEvents|InputAxisInputRight
  (params (AxisValue :type Float%20%28single-precision%29))
  (if (not (Variables|CharacterControl|GetisPressActor))
    (if (Variables|Default|GetisPressMouseRight)
      (Transformation|AddActorWorldOffset (* (* (Math|Transform|TransformDirection (Transformation|GetActorTransform) "0.000000,1.000000, 0") AxisValue) 15.0)))))

(event Input|AxisEvents|InputAxisInputUp
  (params (AxisValue :type Float%20%28single-precision%29))
  (if (not (Variables|CharacterControl|GetisPressActor))
    (if (Variables|Default|GetisPressMouseRight)
      (Transformation|AddActorWorldOffset (* (* (Math|Transform|TransformDirection (Transformation|GetActorTransform) "0.000000,0.000000,1.000000") AxisValue) 15.0)))))