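; BP_ObjectMove is a sphere handle that moves and rotates its parent actor, or itself when it has none.
; Move offsets scale with camera distance; rotation turns the parent's root or the Sphere locally.
; Each Tick grows the Sphere with camera distance, never below unit scale, and the B key toggles its visibility.
; ITransform-named getters expose its transform, forward and right vectors, and rotation.
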(event EventBeginPlay
  (Input|EnableInput (Game|GetPlayerController 0)))

(event Collision|EventActorBeginOverlap
  (params (OtherActor :type Actor%20Object%20Reference)))

(event EventTick
  (params (DeltaSeconds :type Float%20%28single-precision%29))
  (CallFunction|UpdateScalebyCamera))

(event EventSetITransformRotate
  (params (ITransformRotate :type Rotator :default "0, 0, 0") (rotatePower :type Integer))
  (bind _returnvalue (* ITransformRotate rotatePower))
  (bind _returnvalue_2 (Actor|GetParentActor))
  (Utilities|IsValid _returnvalue_2
    (:Is%20Valid
      (Transformation|AddLocalRotation (Variables|/Script/Engine.Actor|GetRootComponent _returnvalue_2) _returnvalue false false))
    (:Is%20Not%20Valid
      (Transformation|AddLocalRotation (Variables|Default|GetSphere) _returnvalue false false))))

(event EventMove
  (params (Direction :type Vector :default "0, 0, 0") (MovePower :type Float%20%28single-precision%29))
  (bind _returnvalue (Actor|GetParentActor))
  (bind _distance (CallFunction|UpdateScalebyDistance))
  (Utilities|IsValid _returnvalue
    (:Is%20Valid
      (Transformation|AddActorWorldOffset _returnvalue (* (* Direction MovePower) _distance)))
    (:Is%20Not%20Valid
      (Transformation|AddActorWorldOffset (* (* Direction MovePower) _distance)))))

(event Input|KeyboardEvents|B
  (params (Key :type Key%20Structure))
  (:Pressed
    (bind _isa (Utilities|FlowControl|FlipFlop)
      (:A
        _)
      (:B
        _))
    (Rendering|SetVisibility (Variables|Default|GetSphere) _isa true)))

(fn ConstructionScript)

(fn UpdateScalebyCamera
  (bind _returnvalue (Game|GetPlayerCameraManager 0))
  (bind _returnvalue_2 (Transformation|GetActorTransform))
  (bind _returnvalue_3 (Transformation|GetActorTransform _returnvalue))
  (bind _location (Math|Transform|BreakTransform _returnvalue_2))
  (bind _location_2 (Math|Transform|BreakTransform _returnvalue_3))
  (bind _returnvalue_4 (Math|Vector|Distance(Vector) _location _location_2))
  (bind _returnvalue_5 (/ _returnvalue_4 2e+03))
  (Transformation|SetWorldScale3D (Variables|Default|GetSphere) (* (Math|Vector|MakeVector 1.0 1.0 1.0) (Math|Float|Clamp(Float) _returnvalue_5 1.0 _returnvalue_5))))

(fn UpdateScalebyDistance
  (return (/ (Math|Vector|Distance(Vector) (.Location (Math|Transform|BreakTransform (Transformation|GetActorTransform))) (.Location (Math|Transform|BreakTransform (Transformation|GetActorTransform (Game|GetPlayerCameraManager 0))))) 1e+02)))

(fn GetITransformTransform
  (return (Transformation|GetActorTransform)))

(fn GetITransformForward
  (return (Transformation|GetActorForwardVector)))

(fn GetITRansformRight
  (return (Transformation|GetActorRightVector)))

(fn GetITransformRotate
  (return (Transformation|GetActorRotation)))